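; Door actor that moves between open and closed positions each time its PlayerActionRayCast event fires.
; It caches its starting location on BeginPlay, then timelines drive SetActorLocation with movement offsets from that point.
; The first activation has its own opening timeline; later ones alternate between close and reopen timelines using IsOpen, with a Complete flag gating those toggles until movement finishes.
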(event EventPlayerActionRayCast
  (params (ActorHit :type Actor%20Object%20Reference) (ComponentHit :type Actor%20Component%20Object%20Reference))
  (if (Variables|Default|GetFirstTime)
    (bind _movement (Timeline|Timeline_2 PlayFromStart)
      (:Update
        _)
      (:Finished
        (Variables|Default|SetComplete true)
        (Variables|Default|SetIsOpen true)))
    (Transformation|SetActorLocation (+ _movement (Variables|Default|GetInitialDoorLocation)) false false)
    (Variables|Default|SetFirstTime false)
    (elif (Variables|Default|GetIsOpen)
      (if (Variables|Default|GetComplete)
        (Variables|Default|SetComplete false)
        (bind _movement_2 (Timeline|Timeline_3 PlayFromStart)
          (:Update
            _)
          (:Finished
            (Variables|Default|SetComplete true)
            (Variables|Default|SetIsOpen false)))
        (Transformation|SetActorLocation (+ _movement_2 (Variables|Default|GetInitialDoorLocation)) false false))
      (elif (Variables|Default|GetComplete)
        (Variables|Default|SetComplete false)
        (bind _movement_3 (Timeline|Timeline_4 PlayFromStart)
          (:Update
            _)
          (:Finished
            (Variables|Default|SetComplete true)
            (Variables|Default|SetIsOpen true)))
        (Transformation|SetActorLocation (+ _movement_3 (Variables|Default|GetInitialDoorLocation)) false false)))))

(event EventBeginPlay
  (Variables|Default|SetInitialDoorLocation (Transformation|GetActorLocation)))

(fn ConstructionScript)