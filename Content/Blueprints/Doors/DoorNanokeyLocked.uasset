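; Locked nanokey door that the player slides open and shut with an interact raycast once it is unlocked.
; A key event unlocks it directly, while a second raycast event spends equipped lockpicks until the required count reaches zero.
; Separate timelines for first open, close and reopen offset the door from its starting location.
; FirstTime, IsOpen and Complete flags choose the timeline and gate later toggles.
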(event EventBeginPlay
  (Variables|Default|SetInitialDoorLocation (Transformation|GetActorLocation)))

(event EventKeytoDoor
  ;[1 1 1] Tells that the door is unlocked
  (Variables|Default|SetIsUnlocked true))

(event EventPlayerActionRayCast
  (params (ActorHit :type Actor%20Object%20Reference) (ComponentHit :type Actor%20Component%20Object%20Reference))
  ;[1 1 1] Checks if this is the first time the door has opened
  (if (Variables|Default|GetFirstTime)
    ;[1 1 1] Checks if unlocked
    (if (Variables|Default|GetIsUnlocked)
      ;[1 1 1] Does anim and tells that its complete when finished
      (bind _movement (Timeline|Timeline_1 PlayFromStart)
        (:Update
          _)
        (:Finished
          (Variables|Default|SetComplete true)
          (Variables|Default|SetIsOpen true)))
      (Transformation|SetActorLocation (+ _movement (Variables|Default|GetInitialDoorLocation)) false false)
      ;[1 1 1] Sets the door to "Open" and tells that everything after won't be the first time
      (Variables|Default|SetFirstTime false))
    (elif (Variables|Default|GetIsUnlocked)
      (if (Variables|Default|GetIsOpen)
        ;[1 1 1] Checks to see if the previous anim is complete
        (if (Variables|Default|GetComplete)
          (Variables|Default|SetComplete false)
          (bind _movement_2 (Timeline|Timeline_2 PlayFromStart)
            (:Update
              _)
            (:Finished
              (Variables|Default|SetComplete true)
              (Variables|Default|SetIsOpen false)))
          (Transformation|SetActorLocation (+ _movement_2 (Variables|Default|GetInitialDoorLocation)) false false))
        (elif (Variables|Default|GetComplete)
          (Variables|Default|SetComplete false)
          (bind _movement_3 (Timeline|Timeline_0 PlayFromStart)
            (:Update
              (Variables|Default|SetComplete true)
              (Variables|Default|SetIsOpen true))
            (:Finished
              _))
          (Transformation|SetActorLocation (+ _movement_3 (Variables|Default|GetInitialDoorLocation)) false false))))))

(event EventPlayerActionRayCast2
  (params (ActorHit :type Actor%20Object%20Reference) (ComponentHit :type Actor%20Component%20Object%20Reference))
  (bind _asfirst_person_character (Utilities|Casting|CastToFirstPersonCharacter (Game|GetPlayerCharacter 0)))
  (if (Variables|/Game/FirstPersonBP/Blueprints/FirstPersonCharacter.FirstPersonCharacter_C|GetLPickEquipped _asfirst_person_character)
    (if (Variables|Default|GetIsPicked)
      (Development|PrintString "You've already picked this lock!")
      (else
        (Variables|Default|SetLPicksNeeded (- (Variables|Default|GetLPicksNeeded) 1))
        (Class|NanokeyDoortoPlayer|NanokeydoortoPlayer(Message) (Game|GetPlayerCharacter 0))
        (if (== 0 (Variables|Default|GetLPicksNeeded))
          (Variables|Default|SetIsPicked true)
          (Development|PrintString "Unlocked!")
          ;[1 1 1] Tells that the door is unlocked
          (Variables|Default|SetIsUnlocked true)
          (else
            (Development|PrintString (Utilities|String|Append (Utilities|String|ToString(Integer) (Variables|Default|GetLPicksNeeded)) " More Lockpicks Needed!"))))))))

(fn ConstructionScript)