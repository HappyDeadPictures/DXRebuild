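; Shotgun actor that serves as world pickup, inventory item and equipped weapon for the first-person character.
; Box overlap shows a pickup widget and enables a raycast action that adds its item struct to the HUD inventory.
; Using it attaches it to the character mesh and sets weapon flags and stats, while Tick hides it when another item is equipped.
; A second raycast action fires bullets from the muzzle, updating ammo after a delay.
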(event OnComponentBeginOverlap(Box)
  (params (OtherActor :type Actor%20Object%20Reference) (OtherComp :type Primitive%20Component%20Object%20Reference) (OtherBodyIndex :type Integer) (bFromSweep :type Boolean) (SweepResult :type Hit%20Result%20Structure%20%28by%20ref%29))
  ;[1 1 1] Overlap pickup text rigger
  (Utilities|Casting|CastToFirstPersonCharacter OtherActor)
  (UserInterface|Viewport|AddtoViewport (Variables|Default|GetPickupTextRef) 0)
  (Variables|Default|SetIsInRange true))

(event OnComponentEndOverlap(Box)
  (params (OtherActor :type Actor%20Object%20Reference) (OtherComp :type Primitive%20Component%20Object%20Reference) (OtherBodyIndex :type Integer))
  ;[1 1 1] Overlap pickup text rigger
  (Utilities|Casting|CastToFirstPersonCharacter OtherActor)
  (Widget|RemovefromParent (Variables|Default|GetPickupTextRef))
  (Variables|Default|SetIsInRange false))

(event Custom|PickupItem_Event_0)

(event EventPlayerActionRayCast2
  (params (ActorHit :type Actor%20Object%20Reference) (ComponentHit :type Actor%20Component%20Object%20Reference))
  (bind _characterref (Variables|Default|GetCharacterRef))
  (bind _characterref_2 (Variables|Default|GetCharacterRef))
  (bind _characterref_3 (Variables|Default|GetCharacterRef))
  ;[1 1 1] Checks ammo count and spawns bullet; Determines reload and firing times
  (Variables|/Game/FirstPersonBP/Blueprints/FirstPersonCharacter.FirstPersonCharacter_C|SetShotgunFiring _characterref_2 true)
  (if (not (< (Variables|/Game/FirstPersonBP/Blueprints/FirstPersonCharacter.FirstPersonCharacter_C|GetAmmoCount _characterref_2) 1))
    (Game|SpawnActorfromClass "/Game/FirstPersonBP/Blueprints/ShotgunBullet.ShotgunBullet_C" (Transformation|GetSocketTransform (Variables|Default|GetEquipped) "Muzzle" "RTS_World") "AlwaysSpawn" 0 0)
    (Audio|PlaySound2D "/Game/Imported/SciFiWeapDark/data/Content/SciFiWeapDark/Sound/Shotgun/Wavs/ShotgunA_Fire01.ShotgunA_Fire01")
    (Utilities|FlowControl|Delay (Variables|Default|GetGunfireTime))
    (Variables|/Game/FirstPersonBP/Blueprints/FirstPersonCharacter.FirstPersonCharacter_C|SetAmmoCount _characterref (- (Variables|/Game/FirstPersonBP/Blueprints/FirstPersonCharacter.FirstPersonCharacter_C|GetAmmoCount _characterref) 1))
    (Variables|/Game/FirstPersonBP/Blueprints/FirstPersonCharacter.FirstPersonCharacter_C|SetShotsFired _characterref (+ (Variables|/Game/FirstPersonBP/Blueprints/FirstPersonCharacter.FirstPersonCharacter_C|GetShotsFired _characterref) 1))
    (Variables|/Game/FirstPersonBP/Blueprints/FirstPersonCharacter.FirstPersonCharacter_C|SetShotgunFiring _characterref_3 false)
    (Variables|/Game/FirstPersonBP/Blueprints/FirstPersonCharacter.FirstPersonCharacter_C|SetShotDone _characterref_3 true)
    (Effects|SpawnEmitteratLocation 0 (Transformation|GetSocketLocation (Variables|Default|GetEquipped) "Muzzle"))))

(event EventUseAction
  (bind _characterref (Variables|Default|GetCharacterRef))
  ;[1 1 1] Equip item
  (Class|Actor|AttachRootComponentto (Variables|/Game/FirstPersonBP/Blueprints/FirstPersonCharacter.FirstPersonCharacter_C|GetMesh2p (Variables|Default|GetCharacterRef)) "Equipped" "SnapToTargetIncludingScale" true)
  (Rendering|SetActorHiddenInGame false)
  (Variables|/Game/Blueprints/UMG/DXGameHUD.DXGameHUD_C|SetIsEquipable (Variables|/Game/FirstPersonBP/Blueprints/FirstPersonCharacter.FirstPersonCharacter_C|GetDXGameHUDRef _characterref) true)
  (Variables|/Game/FirstPersonBP/Blueprints/FirstPersonCharacter.FirstPersonCharacter_C|SetIsEquipped _characterref true)
  (Variables|/Game/FirstPersonBP/Blueprints/FirstPersonCharacter.FirstPersonCharacter_C|SetMaxAmmoCount _characterref (Variables|Default|GetCustomMaxAmmoCount))
  (Variables|/Game/FirstPersonBP/Blueprints/FirstPersonCharacter.FirstPersonCharacter_C|SetReloadDelay _characterref (Variables|Default|GetCustomReloadDelay))
  (Variables|/Game/FirstPersonBP/Blueprints/FirstPersonCharacter.FirstPersonCharacter_C|SetShotgunEquipped _characterref true)
  (Variables|/Game/FirstPersonBP/Blueprints/FirstPersonCharacter.FirstPersonCharacter_C|SetAREquipped _characterref false)
  (Variables|/Game/FirstPersonBP/Blueprints/FirstPersonCharacter.FirstPersonCharacter_C|SetPistolEquipped _characterref false)
  (Variables|/Game/FirstPersonBP/Blueprints/FirstPersonCharacter.FirstPersonCharacter_C|SetMToolEquipped _characterref false)
  (Variables|/Game/FirstPersonBP/Blueprints/FirstPersonCharacter.FirstPersonCharacter_C|SetLPickEquipped _characterref false)
  (Audio|PlaySound2D "/Game/Imported/SciFiWeapDark/data/Content/SciFiWeapDark/Sound/Shotgun/Wavs/Shotgun_Raise.Shotgun_Raise"))

(event EventDropAction
  (params (ItemtoDrop :type Actor%20Object%20Reference))
  (bind _characterref (Variables|Default|GetCharacterRef))
  ;[1 1 1] Removes from inv when dropped
  (Variables|/Game/FirstPersonBP/Blueprints/FirstPersonCharacter.FirstPersonCharacter_C|SetShotguninInv _characterref false)
  (Variables|/Game/FirstPersonBP/Blueprints/FirstPersonCharacter.FirstPersonCharacter_C|SetShotgunEquipped _characterref false)
  (Variables|Default|SetIsInInv false))

(event EventPlayerActionRayCast
  (params (ActorHit :type Actor%20Object%20Reference) (ComponentHit :type Actor%20Component%20Object%20Reference))
  (bind _characterref (Variables|Default|GetCharacterRef))
  (bind _dxgamehudref (Variables|/Game/FirstPersonBP/Blueprints/FirstPersonCharacter.FirstPersonCharacter_C|GetDXGameHUDRef _characterref))
  ;[1 1 1] Removes items from world and adds them to inv refeshs inv
  (if (and (Collision|GetActorEnableCollision) (Variables|Default|GetIsInRange))
    (if (Variables|/Game/FirstPersonBP/Blueprints/FirstPersonCharacter.FirstPersonCharacter_C|GetShotguninInv _characterref)
      (Development|PrintString "You already have this in your inventory!")
      (else
        (Utilities|Array|Add (Variables|/Game/Blueprints/UMG/DXGameHUD.DXGameHUD_C|GetInventory _dxgamehudref) (Variables|Default|GetItemInfo))
        (Variables|/Game/FirstPersonBP/Blueprints/FirstPersonCharacter.FirstPersonCharacter_C|SetShotguninInv _characterref true)
        (Variables|Default|SetIsInInv true)
        (Rendering|SetActorHiddenInGame true)
        (Collision|SetActorEnableCollision false)
        (Development|PrintString (Utilities|String|Append "You Have Acquired a " (Utilities|String|ToString(Text) (Variables|Default|GetCustomPickupText))))
        (Default|RefreshInv _dxgamehudref)))))

(event EventBeginPlay
  (bind _iteminfo (Variables|Default|GetItemInfo))
  (bind (_item _thumbnail _actiontext _pickuptext) (Utilities|Struct|BreakInvStruct _iteminfo))
  ;[1 1 1] Event begin play
  (bind _returnvalue (UserInterface|CreateWidget "/Game/Blueprints/UMG/PickupText.PickupText_C"))
  (Variables|Default|SetPickupTextRef _returnvalue)
  (Utilities|Struct|SetmembersinInvStruct _iteminfo self)
  (Variables|/Game/Blueprints/UMG/PickupText.PickupText_C|SetPickupActor (Variables|Default|GetPickupTextRef) _item)
  (Variables|/Game/Blueprints/UMG/PickupText.PickupText_C|SetPickupText (Variables|Default|GetPickupTextRef) _pickuptext)
  (bind _asfirst_person_character (Utilities|Casting|CastToFirstPersonCharacter (Game|GetPlayerCharacter 0)))
  (bind _output_get (Variables|Default|SetCharacterRef _asfirst_person_character))
  (EventDispatchers|BindEventtoPickupItem _output_get (delegate Custom|PickupItem_Event_0)))

(event EventTick
  (params (DeltaSeconds :type Float%20%28single-precision%29))
  (bind _characterref (Variables|Default|GetCharacterRef))
  ;[1 1 1] Determines whether this is equipped/visible/useable
  (if (Variables|/Game/FirstPersonBP/Blueprints/FirstPersonCharacter.FirstPersonCharacter_C|GetAREquipped _characterref)
    (if (Variables|Default|GetIsInInv) :!label _label
      (Rendering|SetActorHiddenInGame true)
      (Collision|SetActorEnableCollision false))
    (elif (Variables|/Game/FirstPersonBP/Blueprints/FirstPersonCharacter.FirstPersonCharacter_C|GetPistolEquipped _characterref)
      (goto _label)
      (elif (Variables|/Game/FirstPersonBP/Blueprints/FirstPersonCharacter.FirstPersonCharacter_C|GetMToolEquipped _characterref)
        (goto _label)
        (elif (Variables|/Game/FirstPersonBP/Blueprints/FirstPersonCharacter.FirstPersonCharacter_C|GetLPickEquipped _characterref)
          (goto _label))))))

(fn ConstructionScript
  (Utilities|Struct|SetmembersinInvStruct (Variables|Default|GetItemInfo) self (Variables|Default|GetCustomImage) (Variables|Default|GetCustomActionText) (Variables|Default|GetCustomPickupText)))