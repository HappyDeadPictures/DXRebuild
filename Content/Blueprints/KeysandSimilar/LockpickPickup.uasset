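; Lockpick pickup actor that the first-person player can collect into the HUD inventory, equip and use up.
; Box overlap shows a pickup prompt and enables the raycast pickup, which hides the actor and adds its item struct to the inventory.
; Using it attaches it to the character's LPick socket and clears other equip flags.
; Tick polls those flags to hide it when unequipped or destroy it once used.
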(event OnComponentBeginOverlap(Box)
  (params (OtherActor :type Actor%20Object%20Reference) (OtherComp :type Primitive%20Component%20Object%20Reference) (OtherBodyIndex :type Integer) (bFromSweep :type Boolean) (SweepResult :type Hit%20Result%20Structure%20%28by%20ref%29))
  ;[1 1 1] Overlap pickup text rigger
  (Utilities|Casting|CastToFirstPersonCharacter OtherActor)
  (UserInterface|Viewport|AddtoViewport (Variables|Default|GetPickupTextRef) 0)
  (Variables|Default|SetIsInRange true))

(event OnComponentEndOverlap(Box)
  (params (OtherActor :type Actor%20Object%20Reference) (OtherComp :type Primitive%20Component%20Object%20Reference) (OtherBodyIndex :type Integer))
  ;[1 1 1] Overlap pickup text rigger
  (Utilities|Casting|CastToFirstPersonCharacter OtherActor)
  (Widget|RemovefromParent (Variables|Default|GetPickupTextRef))
  (Variables|Default|SetIsInRange false))

(event Custom|PickupItem_Event_0)

(event EventUseAction
  (bind _characterref (Variables|Default|GetCharacterRef))
  ;[1 1 1] Equip item
  (Class|Actor|AttachRootComponentto (Variables|/Game/FirstPersonBP/Blueprints/FirstPersonCharacter.FirstPersonCharacter_C|GetMesh2p (Variables|Default|GetCharacterRef)) "LPick" "SnapToTargetIncludingScale" true)
  (Rendering|SetActorHiddenInGame false)
  (Variables|/Game/Blueprints/UMG/DXGameHUD.DXGameHUD_C|SetIsEquipable (Variables|/Game/FirstPersonBP/Blueprints/FirstPersonCharacter.FirstPersonCharacter_C|GetDXGameHUDRef _characterref) true)
  (Variables|/Game/FirstPersonBP/Blueprints/FirstPersonCharacter.FirstPersonCharacter_C|SetIsEquipped _characterref true)
  (Variables|/Game/FirstPersonBP/Blueprints/FirstPersonCharacter.FirstPersonCharacter_C|SetPistolEquipped _characterref false)
  (Variables|/Game/FirstPersonBP/Blueprints/FirstPersonCharacter.FirstPersonCharacter_C|SetShotgunEquipped _characterref false)
  (Variables|/Game/FirstPersonBP/Blueprints/FirstPersonCharacter.FirstPersonCharacter_C|SetAREquipped _characterref false)
  (Variables|/Game/FirstPersonBP/Blueprints/FirstPersonCharacter.FirstPersonCharacter_C|SetMToolEquipped _characterref false)
  (Variables|/Game/FirstPersonBP/Blueprints/FirstPersonCharacter.FirstPersonCharacter_C|SetLPickEquipped _characterref true))

(event EventDropAction
  (params (ItemtoDrop :type Actor%20Object%20Reference))
  ;[1 1 1] Removes from inv when dropped
  (Variables|/Game/FirstPersonBP/Blueprints/FirstPersonCharacter.FirstPersonCharacter_C|SetLPickEquipped (Variables|Default|GetCharacterRef) false)
  (Variables|Default|SetIsInInv false))

(event EventPlayerActionRayCast
  (params (ActorHit :type Actor%20Object%20Reference) (ComponentHit :type Actor%20Component%20Object%20Reference))
  (bind _characterref (Variables|Default|GetCharacterRef))
  (bind _dxgamehudref (Variables|/Game/FirstPersonBP/Blueprints/FirstPersonCharacter.FirstPersonCharacter_C|GetDXGameHUDRef _characterref))
  ;[1 1 1] Removes items from world and adds them to inv refeshs inv
  (if (and (Collision|GetActorEnableCollision) (Variables|Default|GetIsInRange))
    (Utilities|Array|Add (Variables|/Game/Blueprints/UMG/DXGameHUD.DXGameHUD_C|GetInventory _dxgamehudref) (Variables|Default|GetItemInfo))
    (Variables|Default|SetIsInInv true)
    (Rendering|SetActorHiddenInGame true)
    (Collision|SetActorEnableCollision false)
    (Development|PrintString (Utilities|String|Append "You Have Acquired a " (Utilities|String|ToString(Text) (Variables|Default|GetCustomPickupText))))
    (Default|RefreshInv _dxgamehudref)))

(event EventBeginPlay
  (bind _iteminfo (Variables|Default|GetItemInfo))
  (bind (_item _thumbnail _actiontext _pickuptext) (Utilities|Struct|BreakInvStruct _iteminfo))
  ;[1 1 1] Event begin play
  (bind _returnvalue (UserInterface|CreateWidget "/Game/Blueprints/UMG/PickupText.PickupText_C"))
  (Variables|Default|SetPickupTextRef _returnvalue)
  (Utilities|Struct|SetmembersinInvStruct _iteminfo self)
  (Variables|/Game/Blueprints/UMG/PickupText.PickupText_C|SetPickupActor (Variables|Default|GetPickupTextRef) _item)
  (Variables|/Game/Blueprints/UMG/PickupText.PickupText_C|SetPickupText (Variables|Default|GetPickupTextRef) _pickuptext)
  (bind _asfirst_person_character (Utilities|Casting|CastToFirstPersonCharacter (Game|GetPlayerCharacter 0)))
  (bind _output_get (Variables|Default|SetCharacterRef _asfirst_person_character))
  (EventDispatchers|BindEventtoPickupItem _output_get (delegate Custom|PickupItem_Event_0)))

(event EventTick
  (params (DeltaSeconds :type Float%20%28single-precision%29))
  (bind _characterref (Variables|Default|GetCharacterRef))
  ;[1 1 1] Determines whether this is equipped/visible/useable
  (if (Variables|/Game/FirstPersonBP/Blueprints/FirstPersonCharacter.FirstPersonCharacter_C|GetAREquipped _characterref)
    (if (Variables|Default|GetIsInInv) :!label _label
      (Rendering|SetActorHiddenInGame true)
      (Collision|SetActorEnableCollision false))
    (elif (Variables|/Game/FirstPersonBP/Blueprints/FirstPersonCharacter.FirstPersonCharacter_C|GetShotgunEquipped _characterref)
      (goto _label)
      (elif (Variables|/Game/FirstPersonBP/Blueprints/FirstPersonCharacter.FirstPersonCharacter_C|GetPistolEquipped _characterref)
        (goto _label)
        (elif (Variables|/Game/FirstPersonBP/Blueprints/FirstPersonCharacter.FirstPersonCharacter_C|GetMToolEquipped _characterref)
          (goto _label)
          (elif (Variables|/Game/FirstPersonBP/Blueprints/FirstPersonCharacter.FirstPersonCharacter_C|GetLPickEquipped _characterref)
            ;[1 1 1] Checks ammo count and spawns bullet; Determines reload and firing times
            (if (Variables|Default|GetIsInInv)
              (if (Variables|/Game/FirstPersonBP/Blueprints/FirstPersonCharacter.FirstPersonCharacter_C|GetUsedLPick _characterref)
                (Variables|/Game/FirstPersonBP/Blueprints/FirstPersonCharacter.FirstPersonCharacter_C|SetLPickEquipped _characterref false)
                (Actor|DestroyActor)
                (Class|LockpicktoInv|LockpicktoInv(Message) (Variables|/Game/FirstPersonBP/Blueprints/FirstPersonCharacter.FirstPersonCharacter_C|GetDXGameHUDRef _characterref))
                (Variables|/Game/FirstPersonBP/Blueprints/FirstPersonCharacter.FirstPersonCharacter_C|SetUsedLPick _characterref false)))
            (else
              (goto _label))))))))

(fn ConstructionScript
  (Utilities|Struct|SetmembersinInvStruct (Variables|Default|GetItemInfo) self (Variables|Default|GetCustomImage) (Variables|Default|GetCustomActionText) (Variables|Default|GetCustomPickupText)))