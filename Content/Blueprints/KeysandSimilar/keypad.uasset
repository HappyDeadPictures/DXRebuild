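; Keypad actor that unlocks a linked actor through a four-digit code or by hacking with multitools.
; Raycast hits pass component tags to HitKey, which highlights digit keys via dynamic materials, displays input and handles Clear.
; After four hits, FinishSequence compares the code, turning the indicator red or green and messaging ActorToUnlock on success.
; The second raycast event counts down required multitools, then shares the same unlock path.
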(event Custom|ApendKeysHitInOrder
  (params (KeyHit :type String))
  (Utilities|Array|AppendArray (Variables|Default|GetHitKeysInOrder) (Utilities|Array|MakeArray KeyHit)))

(event Custom|HitKey
  (params (KeyTag :type String))
  (if (not (Variables|Default|GetFinishingSequence))
    (for _array_element (Variables|Default|GetAllKeys)
      (if (Utilities|Enum|Equal(Enum) _array_element KeyTag)
        (Variables|Default|SetHits (+ (Variables|Default|GetHits) 1))
        (if (>= (Utilities|String|Len (Utilities|String|ToString(Text) (Variables|/Script/Engine.TextRenderComponent|GetText (Variables|Default|GetInputKeyTextRender)))) 4)
          (Rendering|Components|TextRender|SetText (Variables|Default|GetInputKeyTextRender) (Variables|Default|GetClearText)))
        (for _index (range 0 9)
          (if (== _index (Math|Conversions|ToInteger(Byte) KeyTag))
            (bind _asstatic_mesh_component (Utilities|Casting|CastToStaticMeshComponent (Utilities|Array|Get(acopy) (Actor|GetComponentsbyTag "/Script/Engine.ActorComponent" (Utilities|String|StringToName (Utilities|String|ToString(Integer) _index))))))
            (CallFunction|UpdateKeyHit _asstatic_mesh_component KeyTag)
            (if (== (Variables|Default|GetHits) 4)
              (Variables|Default|SetFinishingSequence true)
              (Utilities|FlowControl|Delay 0.5)
              (CallFunction|FinishSequence))))
        (elif (Utilities|Enum|Equal(Enum) KeyTag "Clear")
          (CallFunction|ClearInput))))))

(event Custom|FinishSequence
  (bind _indicator (Variables|Default|GetIndicator))
  (if (not (Variables|Default|GetUnlocked))
    (for (_array_element _array_index) (Variables|Default|GetHitKeysInOrder)
      (if (Utilities|Enum|Equal(Enum) _array_element (Utilities|Array|Get(acopy) (Variables|Default|GetCorrectCodeInOrder) _array_index))
        (Variables|Default|SetAmountOfCorrectNumbers (+ (Variables|Default|GetAmountOfCorrectNumbers) 1))))
    (if (== (Variables|Default|GetAmountOfCorrectNumbers) 4)
      (Variables|Default|SetHacked true)
      (Variables|Default|SetUnlocked true)
      (Class|ObjectActionInteraction|ObjectInteraction(Message) (Variables|Default|GetActorToUnlock))
      (Rendering|Material|SetMaterial _indicator 0 "/Game/Imported/Materials/Green.Green")
      (else
        (Variables|Default|SetHits 0)
        (Utilities|Array|Clear (Variables|Default|GetHitKeysInOrder))
        (Rendering|Components|TextRender|SetText (Variables|Default|GetInputKeyTextRender) (Variables|Default|GetClearText))
        (Rendering|Material|SetMaterial _indicator 0 "/Game/Imported/Materials/Red.Red")))
    (Variables|Default|SetAmountOfCorrectNumbers 0)
    (CallFunction|SetNumbersDefaultColor)
    (Variables|Default|SetFinishingSequence false)))

(event Custom|UpdateKeyHit
  (params (Key :type Static%20Mesh%20Component%20Object%20Reference) (KeyNumber :type String))
  (bind _returnvalue (Rendering|Material|CreateDynamicMaterialInstance Key 0 (Rendering|Material|GetMaterial Key 0) :!class /Script/Engine.PrimitiveComponent))
  (Rendering|Material|SetVectorParameterValue _returnvalue "Color" "(R=1.000000,G=1.000000,B=1.000000,A=1.000000)" :!class /Script/Engine.MaterialInstanceDynamic)
  (Rendering|Components|TextRender|SetText (Variables|Default|GetInputKeyTextRender) (Utilities|Text|ToText(String) (Utilities|String|Append (Utilities|String|ToString(Text) (Variables|/Script/Engine.TextRenderComponent|GetText (Variables|Default|GetInputKeyTextRender))) KeyNumber)))
  (CallFunction|ApendKeysHitinOrder KeyNumber))

(event Custom|SetNumbersDefaultColor
  (for _index (range 0 9)
    (bind _asstatic_mesh_component (Utilities|Casting|CastToStaticMeshComponent (Utilities|Array|Get(acopy) (Actor|GetComponentsbyTag "/Script/Engine.ActorComponent" (Utilities|String|StringToName (Utilities|String|ToString(Integer) _index))))))
    (bind _returnvalue (Rendering|Material|CreateDynamicMaterialInstance _asstatic_mesh_component 0 (Rendering|Material|GetMaterial _asstatic_mesh_component 0) :!class /Script/Engine.PrimitiveComponent))
    (Rendering|Material|SetVectorParameterValue :self _returnvalue :!class /Script/Engine.MaterialInstanceDynamic)))

(event Custom|ClearInput
  (if (not (Variables|Default|GetFinishingSequence))
    (Utilities|Array|Clear (Variables|Default|GetHitKeysInOrder))
    (Variables|Default|SetHits 0)
    (Rendering|Components|TextRender|SetText (Variables|Default|GetInputKeyTextRender) (Variables|Default|GetClearText))))

(event EventPlayerActionRayCast
  (params (ActorHit :type Actor%20Object%20Reference) (ComponentHit :type Actor%20Component%20Object%20Reference))
  (CallFunction|HitKey (Utilities|String|ToString(Name) (Utilities|Array|Get(acopy) (Variables|/Script/Engine.ActorComponent|GetComponentTags ComponentHit)))))

(event EventPlayerActionRayCast2
  (params (ActorHit :type Actor%20Object%20Reference) (ComponentHit :type Actor%20Component%20Object%20Reference))
  (bind _asfirst_person_character (Utilities|Casting|CastToFirstPersonCharacter (Game|GetPlayerCharacter 0)))
  (if (Variables|/Game/FirstPersonBP/Blueprints/FirstPersonCharacter.FirstPersonCharacter_C|GetMToolEquipped _asfirst_person_character)
    (if (Variables|Default|GetHacked)
      (Development|PrintString "Terminal Hacked")
      (else
        (Variables|Default|SetMToolsNeeded (- (Variables|Default|GetMToolsNeeded) 1))
        (Class|KeypadtoPlayer|KeypadtoPlayer(Message) (Game|GetPlayerCharacter 0))
        (if (== 0 (Variables|Default|GetMToolsNeeded))
          (Variables|Default|SetHacked true)
          (Variables|Default|SetUnlocked true)
          (Class|ObjectActionInteraction|ObjectInteraction(Message) (Variables|Default|GetActorToUnlock))
          (Rendering|Material|SetMaterial (Variables|Default|GetIndicator) 0 "/Game/Imported/Materials/Green.Green")
          (Variables|Default|SetAmountOfCorrectNumbers 0)
          (CallFunction|SetNumbersDefaultColor)
          (Variables|Default|SetFinishingSequence false)
          (else
            (Development|PrintString (Utilities|String|Append (Utilities|String|ToString(Integer) (Variables|Default|GetMToolsNeeded)) " More Multitools Needed!"))))))))

(fn ConstructionScript
  (Variables|Default|SetAllKeys (Utilities|Array|MakeArray "0" "1" "2" "3" "4" "5" "6" "7" "8" "9")))