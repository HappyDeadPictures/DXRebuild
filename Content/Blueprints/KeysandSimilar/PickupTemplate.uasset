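; Template pickup actor for inventory items that restore the player's health and bio energy.
; The construction script builds its item struct and mesh from custom properties, and a box overlap toggles a prompt widget and in-range flag.
; An in-range raycast action adds the struct to the HUD inventory and hides the actor, keeping it alive until Use applies the bonuses and destroys it.
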(event OnComponentBeginOverlap(Box)
  (params (OtherActor :type Actor%20Object%20Reference) (OtherComp :type Primitive%20Component%20Object%20Reference) (OtherBodyIndex :type Integer) (bFromSweep :type Boolean) (SweepResult :type Hit%20Result%20Structure%20%28by%20ref%29))
  ;[1 1 1] Overlap Pickup Text Trigger
  (Utilities|Casting|CastToFirstPersonCharacter OtherActor)
  (UserInterface|Viewport|AddtoViewport (Variables|Default|GetPickupTextRef) 0)
  (Variables|Default|SetIsInRange true))

(event OnComponentEndOverlap(Box)
  (params (OtherActor :type Actor%20Object%20Reference) (OtherComp :type Primitive%20Component%20Object%20Reference) (OtherBodyIndex :type Integer))
  ;[1 1 1] Overlap Pickup Text Trigger
  (Utilities|Casting|CastToFirstPersonCharacter OtherActor)
  (Widget|RemovefromParent (Variables|Default|GetPickupTextRef))
  (Variables|Default|SetIsInRange false))

(event EventBeginPlay
  (bind _iteminfo (Variables|Default|GetItemInfo))
  (bind (_item _thumbnail _actiontext _pickuptext) (Utilities|Struct|BreakInvStruct _iteminfo))
  ;[1 1 1] Event Begin Play
  (bind _returnvalue (UserInterface|CreateWidget "/Game/Blueprints/UMG/PickupText.PickupText_C"))
  (Variables|Default|SetPickupTextRef _returnvalue)
  (Utilities|Struct|SetmembersinInvStruct _iteminfo self)
  (Variables|/Game/Blueprints/UMG/PickupText.PickupText_C|SetPickupActor (Variables|Default|GetPickupTextRef) _item)
  (Variables|/Game/Blueprints/UMG/PickupText.PickupText_C|SetPickupText (Variables|Default|GetPickupTextRef) _pickuptext)
  (bind _asfirst_person_character (Utilities|Casting|CastToFirstPersonCharacter (Game|GetPlayerCharacter 0)))
  (Variables|Default|SetCharacterRef _asfirst_person_character))

(event EventUseAction
  (bind _characterref (Variables|Default|GetCharacterRef))
  ;[1 1 1] Use Action
  (Variables|/Game/FirstPersonBP/Blueprints/FirstPersonCharacter.FirstPersonCharacter_C|SetHealthValue _characterref (+ (Variables|/Game/FirstPersonBP/Blueprints/FirstPersonCharacter.FirstPersonCharacter_C|GetHealthValue _characterref) (Variables|Default|GetAddHealth)))
  (Variables|/Game/FirstPersonBP/Blueprints/FirstPersonCharacter.FirstPersonCharacter_C|SetBioEnergyValue _characterref (+ (Variables|/Game/FirstPersonBP/Blueprints/FirstPersonCharacter.FirstPersonCharacter_C|GetBioEnergyValue _characterref) (Variables|Default|GetAddBioEnergy)))
  (Variables|/Game/Blueprints/UMG/DXGameHUD.DXGameHUD_C|SetIsEquipable (Variables|/Game/FirstPersonBP/Blueprints/FirstPersonCharacter.FirstPersonCharacter_C|GetDXGameHUDRef (Variables|Default|GetCharacterRef)) false)
  (Actor|DestroyActor))

(event EventPlayerActionRayCast
  (params (ActorHit :type Actor%20Object%20Reference) (ComponentHit :type Actor%20Component%20Object%20Reference))
  (bind _characterref (Variables|Default|GetCharacterRef))
  (bind _dxgamehudref (Variables|/Game/FirstPersonBP/Blueprints/FirstPersonCharacter.FirstPersonCharacter_C|GetDXGameHUDRef _characterref))
  ;[1 1 1] Removes item from world and adds them to inv. Refreshs inv
  (if (and (Collision|GetActorEnableCollision) (Variables|Default|GetIsInRange))
    (Utilities|Array|Add (Variables|/Game/Blueprints/UMG/DXGameHUD.DXGameHUD_C|GetInventory _dxgamehudref) (Variables|Default|GetItemInfo))
    (Widget|RemovefromParent (Variables|Default|GetPickupTextRef))
    (Rendering|SetActorHiddenInGame true)
    (Collision|SetActorEnableCollision false)
    (Development|PrintString (Utilities|String|Append "You Have Acquired a " (Utilities|String|ToString(Text) (Variables|Default|GetCustomPickupText))))
    (Default|RefreshInv _dxgamehudref)))

(fn ConstructionScript
  (Utilities|Struct|SetmembersinInvStruct (Variables|Default|GetItemInfo) self (Variables|Default|GetCustomImage) (Variables|Default|GetCustomActionText) (Variables|Default|GetCustomPickupText))
  (Components|StaticMesh|SetStaticMesh (Variables|Default|GetStaticMesh) (Variables|Default|GetCustomItem)))

(fn GrabInteract
  (params (Player%20aim%20movement :type Vector%202D%20Structure) (Interacting :type Boolean))
  (return "0, 0, 0"))