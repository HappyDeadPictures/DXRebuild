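; BP_LightScultpureDynamic is a light sculpture actor in the Dialog System demo room that spins continuously around its yaw axis.
; The construction script applies the Material variable to the first slot of MeshSculpture.
; Tick adds RotationSpeed scaled by delta time to the actor's yaw, keeping pitch and roll unchanged for frame-rate-independent rotation.
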(event EventTick
  (params (DeltaSeconds :type Float%20%28single-precision%29))
  (bind _returnvalue (Transformation|GetActorRotation))
  (bind (_pitch _yaw _roll) (Class|KismetMathLibrary|BreakRot _returnvalue))
  (Transformation|SetActorRotation (Class|KismetMathLibrary|MakeRot _pitch (+ (* DeltaSeconds (Variables|RotationProperties|GetRotationSpeed)) _yaw) _roll)))

(fn ConstructionScript
  (Rendering|Material|SetMaterial (Variables|Default|GetMeshSculpture) 0 (Variables|Default|GetMaterial)))