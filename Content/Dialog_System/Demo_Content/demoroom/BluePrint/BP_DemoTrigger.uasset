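; BP_DemoTrigger is a trigger button for the Dialog System demo room that relays actor overlaps to a referenced actor.
; The construction script creates a dynamic material instance on one slot of the button mesh.
; Overlap begin and end toggle that material's State parameter and send the matching trigger or end-overlap message to TiggeredActor.
; Overlaps are not filtered by the overlapping actor.
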(event EventActorEndOverlap
  (params (OtherActor :type Actor%20Object%20Reference))
  (Rendering|Material|SetScalarParameterValue (Variables|Default|GetMaterialInstanceButton) "State" 1.0 :!class /Script/Engine.MaterialInstanceDynamic)
  (Class|BPInterfaceButton|CallTriggerActorEndOverlap(Message) (Variables|Default|GetTiggered%20Actor)))

(event EventActorBeginOverlap
  (params (OtherActor :type Actor%20Object%20Reference))
  (Rendering|Material|SetScalarParameterValue (Variables|Default|GetMaterialInstanceButton) "State" 0.0 :!class /Script/Engine.MaterialInstanceDynamic)
  (Class|BPInterfaceButton|CallTriggerActor(Message) (Variables|Default|GetTiggered%20Actor)))

(fn ConstructionScript
  (bind _returnvalue (Rendering|Material|CreateDynamicMaterialInstance (Variables|BP_DemoTrigger|GetButtonMesh) 2 "/Game/Dialog_System/Demo_Content/DemoRoom/Materials/M_Button_Inst.M_Button_Inst" :!class /Script/Engine.PrimitiveComponent))
  (Variables|Default|SetMaterialInstanceButton _returnvalue))